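; Player-driven race car pawn that feeds throttle, steering and handbrake input to its vehicle movement component.
; Input stays disabled from BeginPlay until Tick sees RaceStart on BP_CarController.
; Tick then builds speed and gear strings for the HUD and checks roll, righting a flipped car after a delay.
; Otherwise, a delayed speed check teleports a stopped or reversing car to the Tracker's first checkpoint.
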(event `InputAction|Handbreak`
  (params (Key :type "Key Structure"))
  ;[1 1 1] Input for the car movement
  (:`Pressed`
    (`WheeledVehicleMovementComponent.SetHandbrakeInput` (`self.VehicleMovement`) true))
  (:`Released`
    (`WheeledVehicleMovementComponent.SetHandbrakeInput` (`self.VehicleMovement`) false)))

(event `InputAxis|Throttle`
  (params (AxisValue :type "Float (single-precision)"))
  ;[1 1 1] Input for the car movement
  (`WheeledVehicleMovementComponent.SetThrottleInput` (`self.VehicleMovement`) AxisValue))

(event `InputAxis|Steer`
  (params (AxisValue :type "Float (single-precision)"))
  ;[1 1 1] Input for the car movement
  (`WheeledVehicleMovementComponent.SetSteeringInput` (`self.VehicleMovement`) AxisValue))

(event `self.ReceiveBeginPlay`
  ;[1 1 1] Prevents the car from moving until the countdown ticks down
  (bind _asbp_car_controller (cast `/Game/BP_CarController` (`GameplayStatics.GetPlayerController` 0)))
  (set `self.ControllerRef` _asbp_car_controller)
  (`self.DisableInput` (`self.ControllerRef`)))

(event `Flipped`
  ;[1 1 1] After a short delay flips the car right way up
  (`KismetSystemLibrary.Delay` 5.0)
  (`self.K2_SetActorLocationAndRotation` (+ (`self.K2_GetActorLocation`) (0.0 0.0 5.0) (0.0 0.0 0.0)) (struct) false true))

(event `self.ReceiveTick`
  (params (DeltaSeconds :type "Float (single-precision)"))
  (bind _returnvalue_roll (`KismetMathLibrary.BreakRotator` (`self.K2_GetActorRotation`)))
  (bind _controllerref (`self.ControllerRef`))
  ;[1 1 1] Disables the player input
  (if (`/Game/BP_CarController.RaceStart` _controllerref)
    (`self.EnableInput` _controllerref)
    ;[1 1 1] Update
    (`|ExecutionSequence`
      (:`then_0`
        (set `self.InReverseGear` (< (`WheeledVehicleMovementComponent.GetCurrentGear` (`self.VehicleMovement`)) 0))
        (`self.Update HUD Strings`)
        ;[1 1 1] Checks if the car is upside down
        (bind _output_get (set `self.IsFlipped` (< _returnvalue_roll -80.0)))
        (if _output_get
          (`self.Flipped`)
          (else
            (bind _output_get_2 (set `self.IsFlipped` (> _returnvalue_roll 80.0)))
            (if _output_get_2
              (`self.Flipped`)
              (else
                ;[1 1 1] Reset position to start
                (`KismetSystemLibrary.Delay` 10.0)
                (bind _output_get_3 (set `self.Speed` (`WheeledVehicleMovementComponent.GetForwardSpeed` (`self.VehicleMovement`))))
                (bind _output_get_4 (set `self.IsStopped` (<= _output_get_3 0.0)))
                (if _output_get_4
                  (bind _returnvalue (`GameplayStatics.GetActorOfClass` "/Game/Tracker.Tracker_C"))
                  (`self.K2_SetActorLocationAndRotation` (`self.K2_GetActorLocation` (`|GetArrayItem` (`/Game/Tracker.Checkpoints` _returnvalue))) (struct) false true)
                  (set `self.IsStopped` false))))))))))

(fn `EnableIncarView`
  (params (State :type Boolean))
  (bind _isincar (`self.IsInCar`))
  (set `self.IsInCar` State)
  ;[1 1 1] Update Incar HUD visibilty
  (`SceneComponent.SetVisibility` (`self.InCarGear`) _isincar false)
  (`SceneComponent.SetVisibility` (`self.InCarSpeed`) _isincar false)
  (return))

(fn `Setup Incar HUD`
  ;[1 1 1] Setup Gear Display
  (`TextRenderComponent.K2_SetText` (`self.InCarGear`) (`KismetTextLibrary.Conv_StringToText` (`self.Gear Display String`)))
  (`TextRenderComponent.SetTextRenderColor` (`self.InCarGear`) (`KismetMathLibrary.Conv_LinearColorToColor` (`KismetMathLibrary.SelectColor` (`self.GearDisplayReverseColor`) (`self.GearDisplayColor`) (`self.InReverseGear`))))
  ;[1 1 1] Setup speed display
  (`TextRenderComponent.K2_SetText` (`self.InCarSpeed`) (`KismetTextLibrary.Conv_StringToText` (`self.Speed Display String`))))

(fn `Update HUD Strings`
  (locals (CurrentGear :type Integer))
  (bind _vehiclemovement (`self.VehicleMovement`))
  ;[1 1 1] Setup String for Speed
  (set `self.Speed Display String` (`KismetStringLibrary.Concat_StrStr` (`KismetStringLibrary.Conv_IntToString` (`KismetMathLibrary.FFloor` (`KismetMathLibrary.Abs` (* (`WheeledVehicleMovementComponent.GetForwardSpeed` _vehiclemovement) 0.036)))) " km/h"))
  ;[1 1 1] Setup string for Gear
  (set `local.CurrentGear` (`WheeledVehicleMovementComponent.GetCurrentGear` _vehiclemovement))
  (if (`self.InReverseGear`)
    (set `self.Gear Display String` "R")
    (elif (> (`local.CurrentGear`) 0)
      (set `self.Gear Display String` (`KismetStringLibrary.Conv_IntToString` (`local.CurrentGear`)))
      (else
        (set `self.Gear Display String` "N")))))

(fn `UserConstructionScript`)